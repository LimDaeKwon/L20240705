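; BP_SpawnOverlap is a trigger actor that plays a sound and spawns an object as a VR hand passes through its box.
; BeginPlay assigns a placeholder fire sound, which plays when a VRHandPawn enters the box.
; When that pawn leaves, it spawns BP_SpawnMesh at the first player pawn's transform, shifted along world X rather than the pawn's facing.
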(event `self.ReceiveBeginPlay`
  ;[1 1 1] 음산한거 넣어야함 그냥 대충넣기.
  (`AudioComponent.SetSound` (`self.Audio`) "/Game/VRTemplate/Audio/Fire01.Fire01"))

(event `self.Box.OnComponentBeginOverlap`
  (params (OverlappedComponent :type "PrimitiveComponent Object Reference") (OtherActor :type "Actor Object Reference") (OtherComp :type "PrimitiveComponent Object Reference") (OtherBodyIndex :type Integer) (bFromSweep :type Boolean) (SweepResult :type "HitResult Structure (by ref)"))
  (if (== (`GameplayStatics.GetObjectClass` OtherActor) "/Game/Blueprints/VRHandPawn.VRHandPawn_C")
    (`AudioComponent.Play` (`self.Audio`) 0.0)))

(event `self.Box.OnComponentEndOverlap`
  (params (OverlappedComponent :type "PrimitiveComponent Object Reference") (OtherActor :type "Actor Object Reference") (OtherComp :type "PrimitiveComponent Object Reference") (OtherBodyIndex :type Integer))
  (bind (_returnvalue_location _returnvalue_rotation _returnvalue_scale) (`KismetMathLibrary.BreakTransform` (`self.GetTransform` (`GameplayStatics.GetPlayerPawn` 0))))
  (if (== (`GameplayStatics.GetObjectClass` OtherActor) "/Game/Blueprints/VRHandPawn.VRHandPawn_C")
    (`|SpawnActorFromClass` "/Game/Blueprints/BP_SpawnMesh.BP_SpawnMesh_C" (`KismetMathLibrary.MakeTransform` (+ _returnvalue_location (200.0 0.0 0.0)) _returnvalue_rotation _returnvalue_scale) "Undefined" "MultiplyWithRoot" null null)))

(fn `UserConstructionScript`)